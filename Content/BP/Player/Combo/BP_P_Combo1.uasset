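; Gameplay ability for the first hit of the player's weapon combo, playing the Attack01 section of the weapon attack montage.
; Montage notify windows add and remove gameplay tags: Input toggles Ability.Ready.Combo2 and Branch toggles Ability.Begin.Combo2, gating the second hit.
; The ability ends on montage blend out or interruption, and ending clears only the Begin tag.
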(event Ability|EventActivateAbility
  (Ability|CommitAbility)
  (bind _notifyname (Animation|Montage|PlayMontage (Class|GameplayAbility|GetOwningComponentfromActorInfo) "/Game/BP/Player/Anim/AM_P_WeaponAttack01.AM_P_WeaponAttack01" 1.0 0.0 "Attack01")
    (:OnBlendOut
      (Ability|EndAbility :!label _label))
    (:OnInterrupted
      (goto _label))
    (:OnNotifyBegin
      (switch name _notifyname
        (:Combo1.Input
          (Class|VCBlogComboGameplayAbility|AddGameplayTags "(GameplayTags=((TagName=\"Ability.Ready.Combo2\")))"))
        (:Combo1.Branch
          (Class|VCBlogComboGameplayAbility|AddGameplayTags "(GameplayTags=((TagName=\"Ability.Begin.Combo2\")))"))))
    (:OnNotifyEnd
      (switch name _notifyname
        (:Combo1.Input
          (Class|VCBlogComboGameplayAbility|RemoveGameplayTags "(GameplayTags=((TagName=\"Ability.Ready.Combo2\")))"))
        (:Combo1.Branch
          (Class|VCBlogComboGameplayAbility|RemoveGameplayTags "(GameplayTags=((TagName=\"Ability.Begin.Combo2\")))"))))))

(event Ability|EventOnEndAbility
  (params (bWasCancelled :type Boolean))
  (Class|VCBlogComboGameplayAbility|RemoveGameplayTags "(GameplayTags=((TagName=\"Ability.Begin.Combo2\"),(TagName=\"Ability.Ready.Combo2\")))"))