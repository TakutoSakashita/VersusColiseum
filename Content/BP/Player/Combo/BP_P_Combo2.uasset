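; Gameplay ability for the second attack in the player's weapon combo, playing the Attack02 montage section after committing.
; Montage notify windows Input and Branch add and remove the Combo3 Ready and Begin gameplay tags, opening the chain to the third attack.
; Blend out or interruption ends the ability.
; Ability end clears only the Ready tag, leaving Begin to its notify end.
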(event Ability|EventActivateAbility
  (Ability|CommitAbility)
  (bind _notifyname (Animation|Montage|PlayMontage (Class|GameplayAbility|GetOwningComponentfromActorInfo) "/Game/BP/Player/Anim/AM_P_WeaponAttack02.AM_P_WeaponAttack02" 1.0 0.0 "Attack02")
    (:OnBlendOut
      (Ability|EndAbility :!label _label))
    (:OnInterrupted
      (goto _label))
    (:OnNotifyBegin
      (switch name _notifyname
        (:Combo2.Input
          (Class|VCBlogComboGameplayAbility|AddGameplayTags "(GameplayTags=((TagName=\"Ability.Ready.Combo3\")))"))
        (:Combo2.Branch
          (Class|VCBlogComboGameplayAbility|AddGameplayTags "(GameplayTags=((TagName=\"Ability.Begin.Combo3\")))"))))
    (:OnNotifyEnd
      (switch name _notifyname
        (:Combo2.Input
          (Class|VCBlogComboGameplayAbility|RemoveGameplayTags "(GameplayTags=((TagName=\"Ability.Ready.Combo3\")))"))
        (:Combo2.Branch
          (Class|VCBlogComboGameplayAbility|RemoveGameplayTags "(GameplayTags=((TagName=\"Ability.Begin.Combo3\")))"))))))

(event Ability|EventOnEndAbility
  (params (bWasCancelled :type Boolean))
  (Class|VCBlogComboGameplayAbility|RemoveGameplayTags "(GameplayTags=((TagName=\"Ability.Ready.Combo3\"),(TagName=\"Ability.Begin.Combo3\")))"))